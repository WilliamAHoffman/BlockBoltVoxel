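; Crafter component that fuses loose weapons lying near the user into a new random gun.
; Craft sphere-traces ahead for unpicked weapons, and when at least two are found, sums values over the GunsRequired loop, banks their ammo and destroys them.
; FindDifferences weights each GameMode CraftableGuns class by inverse distance from that total, then spawns a weighted-random pick at the user, favouring similarly valued guns.
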(event `Craft`
  (params (User :type "Actor Object Reference"))
  (bind _returnvalue (`Actor.K2_GetActorLocation` User))
  (set `self.Total Value` 0)
  (set `self.Guns Combine` (`|MakeArray`))
  (bind _outhits (`KismetSystemLibrary.SphereTraceMultiForObjects` :`Start` _returnvalue :`End` (+ _returnvalue (* (`Actor.GetActorForwardVector` User) 150.0)) :`Radius` 150.0 :`ObjectTypes` (`|MakeArray` "ObjectTypeQuery2" :!type "EObjectTypeQuery Enum") :`DrawDebugType` "ForDuration"))
  (for _array_element _outhits
    (bind _asbp_weapon_base (cast `/Game/BluePrints/Weapons/BP_Weapon_Base` (`.HitActor` (`GameplayStatics.BreakHitResult` _array_element))))
    (if (`/Game/BluePrints/Weapons/BP_Weapon_Base.PickedUp` _asbp_weapon_base)
      _
      (elif (not (`KismetArrayLibrary.Array_Contains` (`self.Guns Combine`) _asbp_weapon_base))
        (`KismetArrayLibrary.Array_Add` (`self.Guns Combine`) _asbp_weapon_base))))
  (if (>= (`KismetArrayLibrary.Array_Length` (`self.Guns Combine`)) 2)
    (for _index (range (+ (`self.Guns Required`) 1))
      (bind _output (`|GetArrayItem` (`self.Guns Combine`) _index))
      (set `self.Total Value` (+ (`/Game/BluePrints/Weapons/BP_Weapon_Base.Value` _output) (`self.Total Value`)))
      (bind _asbp_first_person_character (cast `/Game/FirstPerson/Blueprints/BP_FirstPersonCharacter` User))
      (bind _bullets (`/Game/FirstPerson/Blueprints/BP_FirstPersonCharacter.Bullets` _asbp_first_person_character))
      (bind _ammotype (`/Game/BluePrints/Weapons/BP_Weapon_Base.AmmoType` _output))
      (`BlueprintMapLibrary.Map_Add` _bullets _ammotype (+ (`BlueprintMapLibrary.Map_Find` _bullets _ammotype) (`/Game/BluePrints/Weapons/BP_Weapon_Base.CurrentAmmo` _output)))
      (`Actor.K2_DestroyActor` _output))
    (`self.Find Differences`)))

(event `Find Differences`
  (set `self.Random Total` 0.0)
  (set `self.Differences` (`|MakeArray`))
  (bind _asblock_bolt_game_mode (cast `/Game/BlockBoltGameMode` (`GameplayStatics.GetGameMode`)))
  (for _array_element (`/Game/BlockBoltGameMode.Craftable Guns` _asblock_bolt_game_mode)
    (bind _returnvalue (/ 1.0 (+ (`KismetMathLibrary.Abs_Int` (- (`.Value` (defaults `Object` _array_element)) (`self.Total Value`))) 1)))
    (`KismetArrayLibrary.Array_Add` (`self.Differences`) _returnvalue)
    (set `self.Total Differences` (+ _returnvalue (`self.Total Differences`))))
  (set `self.Random Total` (`KismetMathLibrary.RandomFloatInRange` 0.0 (`self.Total Differences`)))
  (for (_array_element_2 _array_index) (`self.Differences`)
    (bind _output_get (set `self.Random Total` (- (`self.Random Total`) _array_element_2)))
    (`KismetSystemLibrary.PrintString` (`KismetStringLibrary.Conv_DoubleToString` _output_get))
    (if (<= _output_get 0.0)
      (bind _asblock_bolt_game_mode_2 (cast `/Game/BlockBoltGameMode` (`GameplayStatics.GetGameMode`)))
      (break)))
  (`|SpawnActorFromClass` (`|GetArrayItem` (`/Game/BlockBoltGameMode.Craftable Guns` _asblock_bolt_game_mode_2) _array_index) (`KismetMathLibrary.MakeTransform` (`Actor.K2_GetActorLocation` (stale `Craft` User))) "Undefined" "MultiplyWithRoot" null null))