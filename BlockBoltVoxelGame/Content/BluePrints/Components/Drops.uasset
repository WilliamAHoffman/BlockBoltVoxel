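; Drops component that spawns weighted random pickups at its owner's location when DropStuff is called.
; The Drops map keys classes to a weight (X) and pickup amount (Y), with EmptyWeight padding the total for no-drop chances.
; The roll repeats inside the weight-summing loop and does not stop at a hit, so several actors can spawn.
; Spawned BP_AmmoUp_Base actors receive their amount through SetPickup.
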(event `Drop Stuff`
  (bind _values (`BlueprintMapLibrary.Map_Values` (`self.Drops`)))
  (for _array_element _values
    (set `self.Total Weight` (+ (`KismetMathLibrary.FTrunc` (`KismetMathLibrary.BreakVector2D` _array_element)) (`self.Total Weight`) (`self.Empty Weight`)))
    (set `self.Random Total` (`KismetMathLibrary.RandomIntegerInRange` 0 (`self.Total Weight`)))
    (bind _keys (`BlueprintMapLibrary.Map_Keys` (`self.Drops`)))
    (for _array_element_2 _keys
      (bind _value (`BlueprintMapLibrary.Map_Find` (`self.Drops`) _array_element_2))
      (set `self.Random Total` (- (`self.Random Total`) (`KismetMathLibrary.BreakVector2D` _value)))
      (if (<= (`self.Random Total`) 0)
        (bind _returnvalue (`|SpawnActorFromClass` _array_element_2 (`KismetMathLibrary.MakeTransform` (`Actor.K2_GetActorLocation` (`self.GetOwner`))) "Undefined" "MultiplyWithRoot" null null))
        (bind _asbp_ammo_up_base (cast `/Game/BluePrints/Pickups/BP_AmmoUp_Base` _returnvalue))
        (`/Game/BluePrints/Pickups/BP_AmmoUp_Base.Set Pickup` _asbp_ammo_up_base (`KismetMathLibrary.FTrunc` (`.Y` (`KismetMathLibrary.BreakVector2D` _value))))
        (`KismetSystemLibrary.PrintString` "drop")
        (else
          (`KismetSystemLibrary.PrintString` "no drop"))))))