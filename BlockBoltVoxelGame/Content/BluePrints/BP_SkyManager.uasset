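; Sky manager that drives a day-night cycle by rotating referenced daylight, night light and sky sphere actors.
; Each tick it adds local pitch scaled by delta time and Cycle to Daylight and SkySphere, and the negated rotation to Nightlight.
; When Daylight is within tolerance of straight up or down pitch, an extra one-degree nudge moves all three past that pole in their respective directions.
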(event `self.ReceiveTick`
  (params (DeltaSeconds :type "Float (single-precision)"))
  (bind _returnvalue (`self.K2_GetActorRotation` (`self.Daylight`)))
  (bind _returnvalue_2 (`KismetMathLibrary.MakeRotator` 0.0 (* DeltaSeconds (`self.Cycle`))))
  (`self.K2_AddActorLocalRotation` (`self.Daylight`) _returnvalue_2 false false)
  (`self.K2_AddActorLocalRotation` (`self.SkySphere`) _returnvalue_2 false false)
  (`self.K2_AddActorLocalRotation` (`self.Nightlight`) (`KismetMathLibrary.NegateRotator` _returnvalue_2) false false)
  (`|ExecutionSequence`
    (:`then_0`
      (if (== _returnvalue (struct :`Pitch` -90.0) :`ErrorTolerance` 1.0)
        (`self.K2_AddActorLocalRotation` (`self.Daylight`) (struct :`Pitch` 1.0) false false)
        (`self.K2_AddActorLocalRotation` (`self.SkySphere`) (struct :`Pitch` 1.0) false false)
        (`self.K2_AddActorLocalRotation` (`self.Nightlight`) (struct :`Pitch` -1.0) false false)))
    (:`then_1`
      (if (== _returnvalue (struct :`Pitch` 90.0) :`ErrorTolerance` 1.0)
        (`self.K2_AddActorLocalRotation` (`self.Daylight`) (struct :`Pitch` 1.0) false false)
        (`self.K2_AddActorLocalRotation` (`self.SkySphere`) (struct :`Pitch` 1.0) false false)
        (`self.K2_AddActorLocalRotation` (`self.Nightlight`) (struct :`Pitch` -1.0) false false)))))

(fn `UserConstructionScript`)