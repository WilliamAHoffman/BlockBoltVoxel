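; Base enemy Blueprint that damages the player on contact, takes damage and awards score when killed.
; HurtStart and HurtStop flag contact with the first-person character and re-arm damage.
; While touching, Tick calls Hurt on the player through BPI_Health, using a CanDamage gate and Delay to space hits.
; Its own Hurt and Heal adjust health; death adds score through BlockBoltGameMode, triggers Drops and destroys the actor.
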(event `Hurt Stop`
  (params (attacked :type "Actor Object Reference"))
  (cast `/Game/FirstPerson/Blueprints/BP_FirstPersonCharacter` attacked)
  (set `self.Touching Target?` false)
  (set `self.Can Damage?` true))

(event `Hurt Start`
  (params (attacked :type "Actor Object Reference"))
  (cast `/Game/FirstPerson/Blueprints/BP_FirstPersonCharacter` attacked)
  (set `self.Touching Target?` true)
  (set `self.Can Damage?` true))

(event `self.ReceiveBeginPlay`
  (set `self.Current Health` (`self.Max Health`))
  (set `self.Target` (`GameplayStatics.GetPlayerPawn` 0)))

(event `self.ReceiveTick`
  (params (DeltaSeconds :type "Float (single-precision)"))
  (if (`self.Touching Target?`)
    (if (`self.Can Damage?`)
      (set `self.Can Damage?` false)
      (bind _asbpi_health (cast `/Game/BluePrints/Interfaces/BPI_Health` (`self.Target`)))
      (`/Game/BluePrints/Interfaces/BPI_Health.Hurt` _asbpi_health (`self.Contact Damage`) null)
      (else
        (`KismetSystemLibrary.Delay` (`self.Damage Delay`))
        (set `self.Can Damage?` true)))))

(event `/Game/BluePrints/Interfaces/BPI_Health.Die`
  (bind _asblock_bolt_game_mode (cast `/Game/BlockBoltGameMode` (`GameplayStatics.GetGameMode`)))
  (`/Game/BlockBoltGameMode.Increase Score` _asblock_bolt_game_mode (`self.Score`))
  (`/Game/BluePrints/Components/Drops.Drop Stuff` (`self.Drops`))
  (`self.K2_DestroyActor`))

(event `/Game/BluePrints/Interfaces/BPI_Health.Hurt`
  (params (amount :type Integer) (cause :type "Actor Object Reference"))
  (bind _output_get (set `self.Current Health` (- (`self.Current Health`) amount)))
  (if (<= _output_get 0)
    (`self.Die`)))

(event `/Game/BluePrints/Interfaces/BPI_Health.Heal`
  (params (amount :type Integer) (cause :type "Actor Object Reference"))
  (set `self.Current Health` (`KismetMathLibrary.Clamp` (+ (`self.Current Health`) amount) 0 (`self.Max Health`))))

(fn `UserConstructionScript`)