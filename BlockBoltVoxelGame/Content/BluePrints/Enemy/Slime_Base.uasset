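; Slime_Base is an enemy base Blueprint that makes a physics-driven slime hop vertically.
; A hit against the VoxelWorld sets OnGround, which lets Tick start a Delay of JumpDelay.
; After the delay it clears OnGround, sets the Cube's vertical velocity to JumpHeight and prints a debug message.
; The jump wires back into the Delay, so hopping repeats without rechecking OnGround.
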(event `self.ReceiveHit`
  (params (MyComp :type "PrimitiveComponent Object Reference") (Other :type "Actor Object Reference") (OtherComp :type "PrimitiveComponent Object Reference") (bSelfMoved :type Boolean) (HitLocation :type "Vector Structure") (HitNormal :type "Vector Structure") (NormalImpulse :type "Vector Structure") (Hit :type "HitResult Structure (by ref)"))
  (cast `VoxelWorld` Other)
  (set `self.On Ground` true))

(event `self.ReceiveTick`
  (params (DeltaSeconds :type "Float (single-precision)"))
  (if (`self.On Ground`)
    (`KismetSystemLibrary.Delay` (`self.Jump Delay`) :!label _label)
    (set `self.On Ground` false)
    (`PrimitiveComponent.SetAllPhysicsLinearVelocity` (`self.Cube`) (`KismetMathLibrary.MakeVector` 0.0 0.0 (`self.Jump Height`)) false)
    (`KismetSystemLibrary.PrintString` "Jump")
    (goto _label)))

(fn `UserConstructionScript`)