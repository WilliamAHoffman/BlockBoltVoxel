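; Base Blueprint for a slime enemy that hops toward its Target and signals hurt start and stop through an overlap box.
; Tick uses Delay nodes to pace a sphere trace at the actor's location, scheduling a jump after JumpDelay when it hits the VoxelWorld.
; Jump sets the physics velocity of Cube0 from the normalized direction to Target scaled by JumpDistance, with JumpHeight as vertical speed.
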(event `Jump`
  (bind (_returnvalue_x _returnvalue_y) (`KismetMathLibrary.BreakVector` (* (`KismetMathLibrary.Normal` (- (`self.K2_GetActorLocation` (`self.Target`)) (`SceneComponent.K2_GetComponentLocation` (`self.Cube_0`)))) (`self.Jump Distance`))))
  (`PrimitiveComponent.SetAllPhysicsLinearVelocity` (`self.Cube_0`) (`KismetMathLibrary.MakeVector` _returnvalue_x _returnvalue_y (`self.Jump Height`)) false))

(event `self.ReceiveTick`
  (params (DeltaSeconds :type "Float (single-precision)"))
  (bind _returnvalue (`self.K2_GetActorLocation`))
  (`parent.ReceiveTick` DeltaSeconds)
  (`KismetSystemLibrary.Delay` 0.2)
  (bind _outhit (`KismetSystemLibrary.SphereTraceSingle` _returnvalue _returnvalue 100.0 "TraceTypeQuery1"))
  (cast `VoxelWorld` (`.HitActor` (`GameplayStatics.BreakHitResult` _outhit)))
  (`KismetSystemLibrary.Delay` (`self.Jump Delay`))
  (`self.Jump`))

(event `self.Box.OnComponentBeginOverlap`
  (params (OverlappedComponent :type "PrimitiveComponent Object Reference") (OtherActor :type "Actor Object Reference") (OtherComp :type "PrimitiveComponent Object Reference") (OtherBodyIndex :type Integer) (bFromSweep :type Boolean) (SweepResult :type "HitResult Structure (by ref)"))
  (`self.Hurt Start` OtherActor))

(event `self.Box.OnComponentEndOverlap`
  (params (OverlappedComponent :type "PrimitiveComponent Object Reference") (OtherActor :type "Actor Object Reference") (OtherComp :type "PrimitiveComponent Object Reference") (OtherBodyIndex :type Integer))
  (`self.Hurt Stop` OtherActor))

(fn `UserConstructionScript`
  (`parent.UserConstructionScript`))