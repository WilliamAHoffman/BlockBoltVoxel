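; Floating enemy Blueprint that homes in on the player and forwards hurt box overlaps to its hurt logic.
; Each Tick, after the parent Tick, it snaps its rotation to face player pawn 0, then moves along its forward vector by Speed scaled by delta time.
; Movement is unswept, so nothing blocks it.
; HurtBox begin and end overlaps call HurtStart and HurtStop with the other actor.
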(event `self.ReceiveTick`
  (params (DeltaSeconds :type "Float (single-precision)"))
  (`parent.ReceiveTick` DeltaSeconds)
  (`|ExecutionSequence`
    (:`then_0`
      (`self.K2_SetActorRotation` (`KismetMathLibrary.FindLookAtRotation` (`self.K2_GetActorLocation`) (`self.K2_GetActorLocation` (`GameplayStatics.GetPlayerPawn` 0)))))
    (:`then_1`
      (`self.K2_AddActorWorldOffset` (* (`self.GetActorForwardVector`) (`self.Speed`) DeltaSeconds)))))

(event `self.Hurt Box.OnComponentBeginOverlap`
  (params (OverlappedComponent :type "PrimitiveComponent Object Reference") (OtherActor :type "Actor Object Reference") (OtherComp :type "PrimitiveComponent Object Reference") (OtherBodyIndex :type Integer) (bFromSweep :type Boolean) (SweepResult :type "HitResult Structure (by ref)"))
  (`self.Hurt Start` OtherActor))

(event `self.Hurt Box.OnComponentEndOverlap`
  (params (OverlappedComponent :type "PrimitiveComponent Object Reference") (OtherActor :type "Actor Object Reference") (OtherComp :type "PrimitiveComponent Object Reference") (OtherBodyIndex :type Integer))
  (`self.Hurt Stop` OtherActor))

(fn `UserConstructionScript`
  (`parent.UserConstructionScript`))