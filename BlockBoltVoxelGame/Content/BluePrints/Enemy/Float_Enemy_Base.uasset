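; Base floating enemy that homes in on the player pawn and deals contact damage.
; Each tick it turns to face the player and moves along its forward vector at Speed without sweeping, so it ignores blocking geometry.
; Overlap with BP_FirstPersonCharacter enables damage through BPI_Health, gated by a delay-based cooldown.
; Its own Hurt event reduces health and destroys the actor at zero.
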(event `self.ReceiveActorBeginOverlap`
  (params (OtherActor :type "Actor Object Reference"))
  (cast `/Game/FirstPerson/Blueprints/BP_FirstPersonCharacter` OtherActor)
  (set `self.Touching Target?` true))

(event `self.ReceiveActorEndOverlap`
  (params (OtherActor :type "Actor Object Reference"))
  (cast `/Game/FirstPerson/Blueprints/BP_FirstPersonCharacter` OtherActor)
  (set `self.Touching Target?` false))

(event `self.ReceiveBeginPlay`
  (set `self.Current Health` (`self.Max Health`))
  (set `self.Target` (`GameplayStatics.GetPlayerPawn` 0)))

(event `self.ReceiveTick`
  (params (DeltaSeconds :type "Float (single-precision)"))
  (`|ExecutionSequence`
    (:`then_0`
      (`self.K2_SetActorRotation` (`KismetMathLibrary.FindLookAtRotation` (`self.K2_GetActorLocation`) (`self.K2_GetActorLocation` (`GameplayStatics.GetPlayerPawn` 0)))))
    (:`then_1`
      (`self.K2_AddActorWorldOffset` (* (`self.GetActorForwardVector`) (`self.Speed`) DeltaSeconds)))
    (:`then_2`
      (if (`self.Touching Target?`)
        (if (`self.Can Damage?`)
          (set `self.Can Damage?` false)
          (bind _asbpi_health (cast `/Game/BluePrints/Interfaces/BPI_Health` (`self.Target`)))
          (`/Game/BluePrints/Interfaces/BPI_Health.Hurt` _asbpi_health (`self.Contact Damage`) null)
          (else
            (`KismetSystemLibrary.Delay` (`self.Damage Cool Down`))
            (set `self.Can Damage?` true)))))))

(event `/Game/BluePrints/Interfaces/BPI_Health.Die`
  (`self.K2_DestroyActor`))

(event `/Game/BluePrints/Interfaces/BPI_Health.Hurt`
  (params (amount :type Integer) (cause :type "Actor Object Reference"))
  (bind _output_get (set `self.Current Health` (- (`self.Current Health`) amount)))
  (if (<= _output_get 0)
    (`self.Die`)))

(fn `UserConstructionScript`)