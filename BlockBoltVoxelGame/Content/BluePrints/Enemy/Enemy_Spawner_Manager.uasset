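; Enemy spawner actor that continuously spawns random enemies around its own location.
; BeginPlay starts a looping Spawn event that waits a random delay between MinDelay and MaxDelay, then spawns a random class from the Enemies array.
; Each spawn lands at a random point in a thin box centered on the actor, sized horizontally by MaxDistance.
; The loop has no stop condition or spawn cap.
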(event `self.ReceiveBeginPlay`
  (`self.Spawn`))

(event `Spawn`
  (`KismetSystemLibrary.Delay` (`KismetMathLibrary.RandomFloatInRange` (`self.Min Delay`) (`self.Max Delay`)) :!label _label)
  (`|SpawnActorFromClass` (`KismetArrayLibrary.Array_Random` (`self.Enemies`)) (`KismetMathLibrary.MakeTransform` (`KismetMathLibrary.RandomPointInBoundingBox` (`self.K2_GetActorLocation`) (`KismetMathLibrary.MakeVector` (`self.Max Distance`) (`self.Max Distance`) 10.0))) "Undefined" "MultiplyWithRoot" null null)
  (goto _label))

(fn `UserConstructionScript`)