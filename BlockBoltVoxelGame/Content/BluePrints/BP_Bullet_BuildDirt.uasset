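; BP_Bullet_BuildDirt is a projectile that builds voxel terrain where it hits a VoxelWorld.
; Both begin and end actor overlaps feed a shared HitObject event, which ignores any other actor type.
; It adds a sphere at the Overlay component's location unless the player pawn is within Radius of the bullet, then destroys itself either way.
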(event `self.ReceiveActorEndOverlap`
  (params (OtherActor :type "Actor Object Reference"))
  (`self.Hit Object` OtherActor))

(event `self.ReceiveActorBeginOverlap`
  (params (OtherActor :type "Actor Object Reference"))
  (`self.Hit Object` OtherActor))

(event `Hit Object`
  (params (`Other Actor` :type "Actor Object Reference"))
  (bind _asvoxel_world (cast `VoxelWorld` `Other Actor`))
  (if (not (< (`self.GetDistanceTo` (`GameplayStatics.GetPlayerPawn` 0)) (`self.Radius`)))
    (`VoxelSphereTools.AddSphere` _asvoxel_world (`SceneComponent.K2_GetComponentLocation` (`self.Overlay`)) (`self.Radius`)))
  (`self.K2_DestroyActor`))

(fn `UserConstructionScript`
  (`parent.UserConstructionScript`))