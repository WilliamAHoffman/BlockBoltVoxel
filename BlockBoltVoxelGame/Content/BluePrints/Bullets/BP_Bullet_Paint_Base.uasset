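; Base paint bullet Blueprint that repaints voxel terrain where it hits.
; On BeginPlay it asks the BlockBolt game mode for the material matching its MaterialChannel and applies it to its cube mesh.
; On a world hit it paints a sphere of that single-index material channel into the voxel world at its location, using its Radius.
; Enemy hits only defer to the parent bullet.
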(event `self.ReceiveBeginPlay`
  (`parent.ReceiveBeginPlay`)
  (bind _asblock_bolt_game_mode (cast `/Game/BlockBoltGameMode` (`GameplayStatics.GetGameMode`)))
  (bind _material (`/Game/BlockBoltGameMode.Get Material from Index` _asblock_bolt_game_mode (`self.Material Channel`)))
  (`PrimitiveComponent.SetMaterial` (`self.Cube`) 0 _material))

(event `self.On Hit World`
  (params (World :type "VoxelWorld Object Reference"))
  (`parent.On Hit World` World)
  (`VoxelSphereTools.SetMaterialSphere` World (`self.K2_GetActorLocation`) (`self.Radius`) (`VoxelBlueprintLibrary.CreateSingleIndexPaintMaterial` (make `VoxelPaintMaterialSingleIndex` (make `VoxelPaintMaterial_MaterialCollectionChannel` (`self.Material Channel`))))))

(event `self.On Hit Enemy`
  (params (Enemy :type "/Game/BluePrints/Interfaces/BPI_Health Interface"))
  (`parent.On Hit Enemy` Enemy))

(fn `UserConstructionScript`
  (`parent.UserConstructionScript`))