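; BP_Bullet_RemoveDirt is a bullet that digs a spherical hole in voxel terrain and drops a dirt ammo pickup.
; Actor overlap feeds HitObject, which ignores anything that is not a VoxelWorld.
; A DoOnce limits it to one hit, which removes the sphere at the bullet's location and spawns BP_AmmoUp_Dirt there carrying AmmoDropAmount.
; The bullet then sets a short life span to destroy itself.
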(event `self.ReceiveActorBeginOverlap`
  (params (OtherActor :type "Actor Object Reference"))
  (`self.Hit Object` OtherActor))

(event `Hit Object`
  (params (`Other Actor` :type "Actor Object Reference"))
  (bind _returnvalue (`self.K2_GetActorLocation`))
  (bind _asvoxel_world (cast `VoxelWorld` `Other Actor`))
  (`/Engine/EditorBlueprintResources/StandardMacros.DoOnce` false
    (:`Completed`
      (`VoxelSphereTools.RemoveSphere` _asvoxel_world _returnvalue (`self.Radius`))
      (bind _returnvalue_2 (`|SpawnActorFromClass` "/Game/BluePrints/Pickups/BP_AmmoUp_Dirt.BP_AmmoUp_Dirt_C" (`KismetMathLibrary.MakeTransform` _returnvalue) "Undefined" "MultiplyWithRoot" null null))
      (set `/Game/BluePrints/Pickups/BP_AmmoUp_Base.Ammo Increase` (`self.Ammo Drop Amount`) _returnvalue_2)
      (`self.SetLifeSpan` 0.1))))

(fn `UserConstructionScript`
  (`parent.UserConstructionScript`))