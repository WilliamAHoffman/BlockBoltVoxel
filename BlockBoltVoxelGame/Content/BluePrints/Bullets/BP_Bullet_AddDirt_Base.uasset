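; BP_Bullet_AddDirt_Base is a bullet Blueprint that adds a sphere of voxel material, dirt by its name, where it hits the voxel world.
; On OnHitWorld it calls AddSphere at the bullet's location, using Radius as the sphere size.
; It skips the edit when player 0's pawn is closer than Radius to the impact, so new terrain is not placed over that pawn's location.
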(event `self.On Hit World`
  (params (World :type "VoxelWorld Object Reference"))
  (if (not (< (`KismetMathLibrary.Vector_Distance` (`self.K2_GetActorLocation`) (`self.K2_GetActorLocation` (`GameplayStatics.GetPlayerPawn` 0))) (`self.Radius`)))
    (`VoxelSphereTools.AddSphere` World (`self.K2_GetActorLocation`) (`self.Radius`))))

(fn `UserConstructionScript`
  (`parent.UserConstructionScript`))