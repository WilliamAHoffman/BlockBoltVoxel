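; Base Blueprint for light bullets that leave a light object behind where they hit.
; It overrides the parent's enemy-hit and world-hit events, calls the parent logic, then routes both into one shared spawn of the LightObject class at the bullet's current location.
; BeginPlay, overlap and Tick are disabled stubs, and the construction script only calls its parent.
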(event `self.On Hit Enemy`
  (params (Enemy :type "/Game/BluePrints/Interfaces/BPI_Health Interface"))
  (`parent.On Hit Enemy` Enemy)
  (`|SpawnActorFromClass` (`self.Light Object`) (`KismetMathLibrary.MakeTransform` (`self.K2_GetActorLocation`)) "Undefined" "MultiplyWithRoot" null null :!label _label))

(event `self.On Hit World`
  (params (World :type "VoxelWorld Object Reference"))
  (`parent.On Hit World` World)
  (goto _label))

(fn `UserConstructionScript`
  (`parent.UserConstructionScript`))