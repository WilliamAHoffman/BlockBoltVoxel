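; Base bullet Blueprint that adds material to the world where it hits, through the BlockBolt game mode.
; On BeginPlay it sets its cube's material to the one the game mode returns for its World tag.
; On a world hit, it calls PlaceAtX at its location using Radius as size, but only when farther than Radius from its Creator.
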(event `self.ReceiveBeginPlay`
  (`parent.ReceiveBeginPlay`)
  (bind _asblock_bolt_game_mode (cast `/Game/BlockBoltGameMode` (`GameplayStatics.GetGameMode`)))
  (bind _material (`/Game/BlockBoltGameMode.Get World Material From Tag` _asblock_bolt_game_mode (`self.World`)))
  (`PrimitiveComponent.SetMaterial` (`self.Cube`) 0 _material))

(event `self.On Hit World`
  (params (World :type "VoxelWorld Object Reference"))
  (`parent.On Hit World` World)
  (if (< (`self.Radius`) (`KismetMathLibrary.Vector_Distance` (`self.K2_GetActorLocation`) (`self.K2_GetActorLocation` (`self.Creator`))))
    (bind _asblock_bolt_game_mode (cast `/Game/BlockBoltGameMode` (`GameplayStatics.GetGameMode`)))
    (`/Game/BlockBoltGameMode.Place at X` _asblock_bolt_game_mode (`self.K2_GetActorLocation`) (`self.Radius`) (`self.World`))))

(fn `UserConstructionScript`
  (`parent.UserConstructionScript`))