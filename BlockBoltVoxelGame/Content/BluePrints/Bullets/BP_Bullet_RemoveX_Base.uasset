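; Base bullet Blueprint that carves a sphere out of a voxel world on impact and drops pickups for the removed material.
; On world hit it paints the sphere with a fixed material index to read back the old materials, tallying them per index in the SpawnDrops map before removing the sphere.
; It then spawns one PickUpDrop per material type, taking the material from BlockBoltGameMode and using the tally as the ammo increase.
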(event `self.On Hit World`
  (params (World :type "VoxelWorld Object Reference"))
  (bind _returnvalue (`self.K2_GetActorLocation`))
  (bind _spawn_drops (`self.Spawn Drops`))
  (bind _spawn_drops_2 (`self.Spawn Drops`))
  (`BlueprintMapLibrary.Map_Clear` (`self.Spawn Drops`))
  (bind _modifiedmaterials (`VoxelSphereTools.SetMaterialSphere` World _returnvalue (`self.Radius`) (`VoxelBlueprintLibrary.CreateSingleIndexPaintMaterial` (make `VoxelPaintMaterialSingleIndex` (make `VoxelPaintMaterial_MaterialCollectionChannel` 39)))))
  (for _array_element _modifiedmaterials
    (bind _returnvalue_2 (`VoxelBlueprintLibrary.GetSingleIndex` (`.OldMaterial` (break `ModifiedVoxelMaterial` _array_element))))
    (`KismetSystemLibrary.PrintString` (`KismetStringLibrary.Conv_ByteToString` _returnvalue_2))
    (bind (_value _returnvalue_3) (`BlueprintMapLibrary.Map_Find` _spawn_drops _returnvalue_2))
    (if _returnvalue_3
      (`BlueprintMapLibrary.Map_Add` _spawn_drops _returnvalue_2 (+ 1 _value))
      (else
        (`BlueprintMapLibrary.Map_Add` _spawn_drops _returnvalue_2 1))))
  (`VoxelSphereTools.RemoveSphere` World _returnvalue (`self.Radius`))
  (bind _keys (`BlueprintMapLibrary.Map_Keys` _spawn_drops_2))
  (for _array_element_2 _keys
    (bind _asblock_bolt_game_mode (cast `/Game/BlockBoltGameMode` (`GameplayStatics.GetGameMode`)))
    (bind _material (`/Game/BlockBoltGameMode.Get Material from Index` _asblock_bolt_game_mode _array_element_2))
    (`|SpawnActorFromClass` (`self.Pick Up Drop`) (`KismetMathLibrary.MakeTransform` (`self.K2_GetActorLocation`)) "Undefined" "MultiplyWithRoot" null _material _array_element_2 (`BlueprintMapLibrary.Map_Find` _spawn_drops_2 _array_element_2) null)))

(fn `UserConstructionScript`
  (`parent.UserConstructionScript`))