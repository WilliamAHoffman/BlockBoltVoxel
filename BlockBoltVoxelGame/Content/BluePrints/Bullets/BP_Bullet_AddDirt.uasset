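; Bullet actor that adds a sphere of terrain ("dirt") to a VoxelWorld it hits.
; Both begin and end overlap route to HitObject, which ignores anything that is not a VoxelWorld.
; It prints the Cube-to-player distance and skips AddSphere at the Overlay position when that distance is under Radius.
; The bullet destroys itself after any voxel-world hit, whether or not terrain is added.
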(event `self.ReceiveActorBeginOverlap`
  (params (OtherActor :type "Actor Object Reference"))
  (`self.Hit Object` OtherActor))

(event `self.ReceiveActorEndOverlap`
  (params (OtherActor :type "Actor Object Reference"))
  (`self.Hit Object` OtherActor))

(event `Hit Object`
  (params (`Other Actor` :type "Actor Object Reference"))
  (bind _returnvalue (`KismetMathLibrary.Vector_Distance` (`SceneComponent.K2_GetComponentLocation` (`self.Cube`)) (`self.K2_GetActorLocation` (`GameplayStatics.GetPlayerPawn` 0))))
  (bind _asvoxel_world (cast `VoxelWorld` `Other Actor`))
  (`KismetSystemLibrary.PrintString` (`KismetStringLibrary.Conv_DoubleToString` _returnvalue))
  (if (not (< _returnvalue (`self.Radius`)))
    (`VoxelSphereTools.AddSphere` _asvoxel_world (`SceneComponent.K2_GetComponentLocation` (`self.Overlay`)) (`self.Radius`)))
  (`self.K2_DestroyActor`))

(fn `UserConstructionScript`
  (`parent.UserConstructionScript`))