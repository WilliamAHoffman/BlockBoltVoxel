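; Base Blueprint for build guns, weapons that fire AddX bullets and use inventory material as ammo.
; It overrides bullet spawning to pass radius, the selected material channel and motion and damage parameters to the projectile.
; Ammo checks and deductions go through BlockBoltGameMode, drawing AmmoPerShot units of the current material channel, which can be changed through an event.
; Firing and construction defer to the parent class.
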(event `self.Fire`
  (params (Shooter :type "Actor Object Reference"))
  (`parent.Fire` Shooter))

(event `self.Spawn Bullet`
  (params (Shooter :type "Actor Object Reference") (Location :type "Vector Structure") (Rotation :type "Rotator Structure") (Speed :type "Float (double-precision)") (Damage :type Integer) (Acceleration :type "Float (double-precision)") (`Homing Magnitude` :type "Float (double-precision)"))
  (`|SpawnActorFromClass` "/Game/BluePrints/Bullets/BP_Bullet_AddX_Base.BP_Bullet_AddX_Base_C" (`KismetMathLibrary.MakeTransform` Location Rotation) "Undefined" "MultiplyWithRoot" null (`self.Radius`) (`self.Material Channel`) Speed Damage Shooter Acceleration `Homing Magnitude` null))

(event `/Game/BluePrints/Interfaces/BPI_Select_Materials.Set Material Channel`
  (params (Channel :type Byte))
  (set `self.Material Channel` Channel))

(fn `Can Reduce Ammo?`
  (returns (`Success?` :type Boolean))
  (bind _asblock_bolt_game_mode (cast `/Game/BlockBoltGameMode` (`GameplayStatics.GetGameMode`)))
  (bind _result (`/Game/BlockBoltGameMode.Has Enough Material?` _asblock_bolt_game_mode (`self.Material Channel`) (`self.AmmoPerShot`)))
  (return _result))

(fn `Reduce Ammo`
  (bind _asblock_bolt_game_mode (cast `/Game/BlockBoltGameMode` (`GameplayStatics.GetGameMode`)))
  (`/Game/BlockBoltGameMode.Remove From Inventory` _asblock_bolt_game_mode (`self.Material Channel`) (`self.AmmoPerShot`)))

(fn `UserConstructionScript`
  (`parent.UserConstructionScript`))