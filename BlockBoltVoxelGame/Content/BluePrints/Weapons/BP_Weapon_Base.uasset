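; Base weapon actor that can be picked up into a character's inventory, dropped, fired and reloaded, with pickup state toggling its sphere collision.
; Fire spends magazine ammo and spawns one or more bullet actors ahead of the shooter, aimed along player 0's camera with random spread, using a delay to limit fire rate.
; After a delay, Reload refills the magazine from the character's per-ammo-type bullet map and updates their text.
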(event `/Game/BluePrints/Interfaces/BPI_Item.Drop`
  (set `self.PickedUp` false)
  (`PrimitiveComponent.SetCollisionEnabled` (`self.Sphere`) "QueryAndPhysics"))

(event `/Game/BluePrints/Interfaces/BPI_Item.Pick Up`
  (set `self.PickedUp` true)
  (`PrimitiveComponent.SetCollisionEnabled` (`self.Sphere`) "NoCollision"))

(event `/Game/BluePrints/Interfaces/BPI_Item.Pick Up Attempt`
  (params (Character :type "/Game/FirstPerson/Blueprints/BP_FirstPersonCharacter Object Reference"))
  (if (not (`self.PickedUp`))
    (`/Game/FirstPerson/Blueprints/BP_FirstPersonCharacter.Add To Invetory` Character self)))

(event `Fire`
  (params (Shooter :type "Actor Object Reference"))
  (bind _returnvalue (`GameplayStatics.GetPlayerCameraManager` 0))
  (bind _spread (`self.Spread`))
  (bind (_returnvalue_roll _returnvalue_pitch _returnvalue_yaw) (`KismetMathLibrary.BreakRotator` (`PlayerCameraManager.GetCameraRotation` _returnvalue)))
  (bind _returnvalue_2 (* _spread -1.0))
  (if (`self.Reloading`)
    _
    (elif (`self.Can Fire`)
      (if (>= (`self.CurrentAmmo`) (`self.AmmoPerShot`))
        (set `self.CurrentAmmo` (- (`self.CurrentAmmo`) (`self.AmmoPerShot`)))
        (for _ (range 1 (+ (`self.Shot Count`) 1))
          (`|SpawnActorFromClass` (`self.Bullet`) (`KismetMathLibrary.MakeTransform` (+ (`self.K2_GetActorLocation` Shooter) (* (`self.GetActorForwardVector` _returnvalue) 100.0) (0.0 0.0 0.0)) (`KismetMathLibrary.MakeRotator` (+ _returnvalue_roll (`KismetMathLibrary.RandomFloatInRange` _returnvalue_2 _spread)) (+ _returnvalue_pitch (`KismetMathLibrary.RandomFloatInRange` _returnvalue_2 _spread)) (+ _returnvalue_yaw (`KismetMathLibrary.RandomFloatInRange` _returnvalue_2 _spread)))) "Undefined" "MultiplyWithRoot" null Shooter null)
          (set `self.Can Fire` false)
          (`KismetSystemLibrary.Delay` (`self.Delay`))
          (set `self.Can Fire` true))))))

(event `Reload`
  (params (Character :type "/Game/FirstPerson/Blueprints/BP_FirstPersonCharacter Object Reference"))
  (bind _bullets (`/Game/FirstPerson/Blueprints/BP_FirstPersonCharacter.Bullets` Character))
  (bind _ammotype (`self.AmmoType`))
  (bind _ammo_used (`self.Ammo Used`))
  (bind _value (`BlueprintMapLibrary.Map_Find` _bullets (`self.AmmoType`)))
  (if (not (`self.Reloading`))
    (set `self.Reloading` true)
    (`KismetSystemLibrary.Delay` (`self.Reload Delay`))
    (if (> _value 0)
      (bind _output_get (set `self.Ammo Used` (- (`self.MagSize`) (`self.CurrentAmmo`))))
      (if (> _output_get 0)
        (bind _output_get_2 (set `self.Ammo Used` (`KismetMathLibrary.Clamp` _value 0 (- (`self.MagSize`) (`self.CurrentAmmo`)))))
        (`KismetSystemLibrary.PrintString` (`KismetStringLibrary.Conv_IntToString` _output_get_2))
        (set `self.CurrentAmmo` (+ (`self.CurrentAmmo`) _ammo_used))
        (`BlueprintMapLibrary.Map_Add` _bullets _ammotype (- (`BlueprintMapLibrary.Map_Find` _bullets _ammotype) _ammo_used))
        (set `self.Reloading` false)
        (`/Game/FirstPerson/Blueprints/BP_FirstPersonCharacter.Update Text` Character)
        (else
          (set `self.Reloading` false)))
      (else
        (set `self.Reloading` false)))))

(fn `Get Item Texture`
  (returns (Texture :type "Texture2D Object Reference"))
  (return (`self.Texture`)))

(fn `UserConstructionScript`)