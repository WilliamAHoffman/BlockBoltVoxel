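; Base weapon Blueprint that fires projectiles at a limited rate.
; Fire spawns the configurable BulletType just ahead of the actor, rotated to the player 0 camera, and prints the actor's location.
; A CanFire flag blocks further shots until the Delay interval elapses.
; Reload and CheckAmmoReload are empty stubs, so no ammo logic runs here.
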(event `Fire`
  (bind _returnvalue (`self.K2_GetActorLocation`))
  (if (`self.Can Fire`)
    (`KismetSystemLibrary.PrintString` (`KismetStringLibrary.Conv_VectorToString` _returnvalue))
    (`|SpawnActorFromClass` (`self.BulletType`) (`KismetMathLibrary.MakeTransform` (+ _returnvalue (* (`self.GetActorForwardVector`) 100.0)) (`PlayerCameraManager.GetCameraRotation` (`GameplayStatics.GetPlayerCameraManager` 0))) "Undefined" "MultiplyWithRoot" null null)
    (set `self.Can Fire` false)
    (`KismetSystemLibrary.Delay` (`self.Delay`))
    (set `self.Can Fire` true)))

(event `Reload`
  (params (AmmoIn :type Integer)))

(fn `Check Ammo Reload`)

(fn `UserConstructionScript`)