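; BP_AmmoUp_Build is an ammo pickup that adds to the player's inventory on contact.
; BeginPlay runs the parent logic, then applies MaterialWorld to the Cube.
; When BP_FirstPersonCharacter overlaps it, it passes Type and AmmoIncrease to BlockBoltGameMode's AddToInventory, then destroys itself.
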(event `self.ReceiveBeginPlay`
  (`parent.ReceiveBeginPlay`)
  (`PrimitiveComponent.SetMaterial` (`self.Cube`) 0 (`self.Material World`)))

(event `self.ReceiveActorBeginOverlap`
  (params (OtherActor :type "Actor Object Reference"))
  (cast `/Game/FirstPerson/Blueprints/BP_FirstPersonCharacter` OtherActor)
  (bind _asblock_bolt_game_mode (cast `/Game/BlockBoltGameMode` (`GameplayStatics.GetGameMode`)))
  (`/Game/BlockBoltGameMode.Add To Inventory` _asblock_bolt_game_mode (`self.Type`) (`self.Ammo Increase`))
  (`self.K2_DestroyActor`))

(fn `UserConstructionScript`
  (`parent.UserConstructionScript`))