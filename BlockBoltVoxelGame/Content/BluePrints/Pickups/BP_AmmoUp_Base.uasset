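; BP_AmmoUp_Base is an ammo pickup, apparently a base class, that adds ammo to the first-person character and expires after its configured lifetime.
; On the first overlap with BP_FirstPersonCharacter, guarded by a DoOnce, it disables the Cube's physics and collision and calls IncreaseAmmo with its AmmoIncrease and AmmoType values.
; It then removes itself by shortening its life span rather than destroying the actor directly.
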(event `self.ReceiveBeginPlay`
  (`self.SetLifeSpan` (`self.LifeTime`)))

(event `self.ReceiveActorBeginOverlap`
  (params (OtherActor :type "Actor Object Reference"))
  (bind _asbp_first_person_character (cast `/Game/FirstPerson/Blueprints/BP_FirstPersonCharacter` OtherActor))
  (`/Engine/EditorBlueprintResources/StandardMacros.DoOnce` false
    (:`Completed`
      (`PrimitiveComponent.SetSimulatePhysics` (`self.Cube`) false)
      (`PrimitiveComponent.SetCollisionEnabled` (`self.Cube`) "NoCollision")
      (`/Game/FirstPerson/Blueprints/BP_FirstPersonCharacter.Increase Ammo` _asbp_first_person_character (`self.Ammo Increase`) (`self.Ammo Type`))
      (`self.SetLifeSpan` 0.1))))

(fn `UserConstructionScript`)